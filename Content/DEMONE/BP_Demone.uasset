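; Demone enemy character that patrols random reachable points, then chases and melees the player when its sight component spots them.
; AIMoveTo drives patrol and pursuit, looping the attack montage while the player stays close.
; Montage notifies toggle the attack hitbox and reset a DoOnce that limits overlap damage per swing.
; Incoming damage updates a widget health bar, interrupts with a hit montage, or plays death and destroys the actor.
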(event OnSeePawn(Vista)
  (params (Pawn :type Pawn%20Object%20Reference))
  (bind _asbp_third_person_character (Utilities|Casting|CastToBP_ThirdPersonCharacter Pawn))
  (if (Variables|/Game/ThirdPerson/Blueprints/BP_ThirdPersonCharacter.BP_ThirdPersonCharacter_C|GetE_Morto? _asbp_third_person_character)
    (Components|Movement|StopMovementImmediately (Variables|Character|GetCharacterMovement))
    (CallFunction|Ronda)
    (elif (not (Variables|Default|GetStaInseguendo?))
      (Variables|Default|SetStaInseguendo? true)
      (Variables|/Script/Engine.CharacterMovementComponent|SetMaxWalkSpeed (Variables|Character|GetCharacterMovement) 6e+02)
      (AI|AIMoveTo self "0, 0, 0" _asbp_third_person_character 1.2e+02 false :!label _label
        (:OnSuccess
          (bind _notifyname (Animation|Montage|PlayMontage (Variables|Character|GetMesh) "/Game/DEMONE/AM_AttaccoDemone.AM_AttaccoDemone" :!label _label_2)
            (:OnCompleted
              (if (<= (Transformation|GetDistanceTo self _asbp_third_person_character) 3e+02)
                (Utilities|FlowControl|Delay 0.5)
                (goto _label_2)
                (else
                  (goto _label))))
            (:OnNotifyBegin
              (if (== _notifyname "AttivaDanno")
                (Collision|SetCollisionEnabled (Variables|Default|GetHitbox_Attacco) "QueryAndPhysics")
                (Utilities|FlowControl|DoOnce false) ; enters at Reset
                (elif (== _notifyname "DisattivaDanno")
                  (Collision|SetCollisionEnabled (Variables|Default|GetHitbox_Attacco) "NoCollision"))))))
        (:OnFail
          (Variables|Default|SetStaInseguendo? false)
          (Variables|/Script/Engine.CharacterMovementComponent|SetMaxWalkSpeed (Variables|Character|GetCharacterMovement) 3e+02)
          (CallFunction|Ronda))))))

(event OnComponentBeginOverlap(Hitbox_Attacco)
  (params (OverlappedComponent :type Primitive%20Component%20Object%20Reference) (OtherActor :type Actor%20Object%20Reference) (OtherComp :type Primitive%20Component%20Object%20Reference) (OtherBodyIndex :type Integer) (bFromSweep :type Boolean) (SweepResult :type Hit%20Result%20Structure%20%28by%20ref%29))
  (bind _asbp_third_person_character (Utilities|Casting|CastToBP_ThirdPersonCharacter OtherActor))
  (Utilities|FlowControl|DoOnce false
    (:Completed
      (Game|Damage|ApplyDamage _asbp_third_person_character 15.0 0 self))))

(event Custom|Ronda
  (if (not (Variables|Default|GetStaInseguendo?))
    (Variables|/Script/Engine.CharacterMovementComponent|SetMaxWalkSpeed (Variables|Character|GetCharacterMovement) 3e+02)
    (AI|AIMoveTo self (.RandomLocation (AI|Navigation|GetRandomReachablePointinRadius (Transformation|GetActorLocation) 1.5e+03 0 0)) 0 5.0 false
      (:OnSuccess
        (Utilities|FlowControl|Delay 2.5))
      (:OnFail
        (Utilities|FlowControl|Delay 1.0)))
    (CallFunction|Ronda)))

(event EventBeginPlay
  (CallFunction|Ronda)
  (Utilities|FlowControl|Sequence
    (:then_1
      (bind _aswbp_vita (Utilities|Casting|CastToWBP_Vita (UserInterface|GetUserWidgetObject (Variables|Default|GetWidget_Vita))))
      (Progress|SetPercent (Variables|/Game/WBP_Vita.WBP_Vita_C|GetBarraVerde _aswbp_vita) 1.0))))

(event Collision|EventActorBeginOverlap
  (params (OtherActor :type Actor%20Object%20Reference)))

(event EventTick
  (params (DeltaSeconds :type Float%20%28single-precision%29)))

(event Game|Damage|EventAnyDamage
  (params (Damage :type Float%20%28single-precision%29) (DamageType :type Damage%20Type%20Object%20Reference) (InstigatedBy :type Controller%20Object%20Reference) (DamageCauser :type Actor%20Object%20Reference))
  (bind _output_get (Variables|Default|SetVita (Math|Float|Clamp(Float) (- (Variables|Default|GetVita) Damage) 0.0 1e+02)))
  (bind _aswbp_vita (Utilities|Casting|CastToWBP_Vita (UserInterface|GetUserWidgetObject (Variables|Default|GetWidget_Vita))))
  (Progress|SetPercent (Variables|/Game/WBP_Vita.WBP_Vita_C|GetBarraVerde _aswbp_vita) (/ (Variables|Default|GetVita) 1e+02))
  (if (<= _output_get 0.0)
    (Animation|StopAnimMontage 0)
    (Collision|SetCollisionEnabled (Variables|Default|GetHitbox_Attacco) "NoCollision")
    (Pawn|Components|CharacterMovement|DisableMovement (Variables|Character|GetCharacterMovement))
    (Components|Animation|SetAnimationMode (Variables|Character|GetMesh) "AnimationSingleNode" false)
    (Components|Animation|PlayAnimation (Variables|Character|GetMesh) "/Game/DEMONE/Falling_Forward_Death.Falling_Forward_Death" false)
    (Utilities|FlowControl|Delay 2.0)
    (Components|DestroyComponent (Variables|Default|GetWidget_Vita))
    (Actor|DestroyActor)
    (else
      (Animation|StopAnimMontage 0)
      (Animation|Montage|PlayMontage (Variables|Character|GetMesh) "/Game/DEMONE/AM_Demone_Hit.AM_Demone_Hit"
        (:OnCompleted
          _)
        (:OnInterrupted
          _))
      (Variables|Default|SetStaInseguendo? false))))

(fn ConstructionScript)