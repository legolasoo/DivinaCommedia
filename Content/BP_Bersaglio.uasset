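; BP_Bersaglio is a target actor with health that takes damage and is destroyed when its health runs out.
; The SubisciDanno event decrements Vita and updates the green progress bar in its WBP_Vita widget component as a fraction of three.
; While health remains, the cube briefly flashes red through a delayed material swap back to the default.
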(event Custom|SubisciDanno
  (bind _output_get (Variables|Default|SetVita (- (Variables|Default|GetVita) 1)))
  (bind _aswbp_vita (Utilities|Casting|CastToWBP_Vita (UserInterface|GetUserWidgetObject (Variables|Default|GetWBP_Vita))))
  (Progress|SetPercent (Variables|/Game/WBP_Vita.WBP_Vita_C|GetBarraVerde _aswbp_vita) (/ (Math|Conversions|ToFloat(Integer) (Variables|Default|GetVita)) 3.0))
  (if (<= _output_get 0)
    (Actor|DestroyActor)
    (else
      (Rendering|Material|SetMaterial (Variables|Default|GetCube) 0 "/Game/M_Rosso.M_Rosso")
      (Utilities|FlowControl|Delay 0.2)
      (Rendering|Material|SetMaterial (Variables|Default|GetCube) 0 "/Game/LevelPrototyping/Materials/MI_DefaultColorway.MI_DefaultColorway"))))

(event EventBeginPlay)

(event Collision|EventActorBeginOverlap
  (params (OtherActor :type Actor%20Object%20Reference)))

(event EventTick
  (params (DeltaSeconds :type Float%20%28single-precision%29)))

(fn ConstructionScript)